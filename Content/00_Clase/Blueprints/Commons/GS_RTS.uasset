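; GS_RTS is the RTS game state that shares player cursors and spawns buildings and units for players.
; A looping timer gathers each controller's ID, name, color and cursor position, then passes the list to every controller's OtherCursors.
; Spawn events create base building or unit actors owned by the requesting controller.
; GetPlayerControllers caches PC_RTS references, rebuilding them when the count differs from PlayerArray.
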(event Custom|SyncPlayersCursor
  (bind _as_pc_rts (CallFunction|GetPlayerControllers))
  (Utilities|Array|Clear (Variables|Default|GetPlayer%20Data))
  (for _array_element _as_pc_rts
    (Utilities|Array|Add (Variables|Default|GetPlayer%20Data) (Utilities|Struct|MakeS_PlayerData (.id (Variables|/Game/00_Clase/Blueprints/Commons/PC_RTS.PC_RTS_C|GetPlayer%20Data _array_element)) (.name (Variables|/Game/00_Clase/Blueprints/Commons/PC_RTS.PC_RTS_C|GetPlayer%20Data _array_element)) (.color (Variables|/Game/00_Clase/Blueprints/Commons/PC_RTS.PC_RTS_C|GetPlayer%20Data _array_element)) (Variables|/Game/00_Clase/Blueprints/Commons/PC_RTS.PC_RTS_C|GetCursorPosition _array_element))))
  (bind _as_pc_rts_2 (CallFunction|GetPlayerControllers))
  (for _array_element_2 _as_pc_rts_2
    (Default|OtherCursors _array_element_2 (Variables|Default|GetPlayer%20Data))))

(event Custom|SpawnBuildForPlayer
  (params (PC :type PC%20RTS%20Object%20Reference) (ID%20Building :type Name) (Location :type Vector) (ColorPlayer :type Linear%20Color%20Structure))
  (Game|SpawnActorfromClass "/Game/00_Clase/Blueprints/Buildings/BP_BaseDefinitiveBuilding.BP_BaseDefinitiveBuilding_C" (Math|Transform|MakeTransform Location "0, 0, 0" "1.000000,1.000000,1.000000") "Undefined" "MultiplyWithRoot" PC ID%20Building ColorPlayer (Pawn|GetControlledPawn PC)))

(event Custom|SpawnUnitForPlayer
  (params (PC%20RTS :type PC%20RTS%20Object%20Reference) (ID%20Unit :type Name) (Spawn%20Transform%20Location :type Vector) (RallyPoint :type Vector))
  (Game|SpawnActorfromClass "/Game/00_Clase/Blueprints/Units/BP_BaseUnit.BP_BaseUnit_C" (Math|Transform|MakeTransform Spawn%20Transform%20Location "0, 0, 0" "1.000000,1.000000,1.000000") "Undefined" "MultiplyWithRoot" PC%20RTS ID%20Unit RallyPoint (Pawn|GetControlledPawn PC%20RTS)))

(event EventBeginPlay
  (Utilities|Time|SetTimerbyEvent (delegate Custom|SyncPlayersCursor) 0.1 true))

(fn ConstructionScript)

(fn GetPlayerControllers
  (if (== (Utilities|Array|Length (Variables|Default|GetPlayerArray)) (Utilities|Array|Length (Variables|Default|GetAs%20PC%20RTS)))
    (return (Variables|Default|GetAs%20PC%20RTS))
    (else
      (Utilities|Array|Clear (Variables|Default|GetAs%20PC%20RTS))
      (for _array_element (Variables|Default|GetPlayerArray)
        (bind _aspc_rts (Utilities|Casting|CastToPC_RTS (Game|GetPlayerController _array_element)))
        (Utilities|Array|Add (Variables|Default|GetAs%20PC%20RTS) _aspc_rts))
      (return (Variables|Default|GetAs%20PC%20RTS)))))