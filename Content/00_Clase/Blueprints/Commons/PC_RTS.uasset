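; RTS player controller that sets up input, custom cursor, per-player data and a starting town hall in a multiplayer match.
; It relays HUD updates and orders to the pawn, and handles building previews, resource-checked crafting and rally points, with construction created through the game state.
; A looping timer and cursor events share positions to show other players' cursors.
; Cached getters resolve framework references, and hardcoded numpad keys trigger building previews and villager spawning.
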(event Custom|AddMappingContext
  (Utilities|FlowControl|Delay 0.2)
  (Input|AddMappingContext (PlayerController|LocalPlayerSubsystems|GetEnhancedInputLocalPlayerSubsystem) "/Game/00_Clase/Input/IMC_Pawn.IMC_Pawn" 0 "(bIgnoreAllPressedKeysUntilRelease=True,bForceImmediately=False,bNotifyUserSettings=False)"))

(event Custom|SetDataPlayersOnServer
  (params (Data%20Player :type S%20Player%20Data%20Structure))
  (Variables|Default|SetPlayer%20Data Data%20Player))

(event Custom|SaveCursorPosition
  (bind _location (CallFunction|GetCursorPosition "TraceTypeQuery1"))
  (bind _output_get (Variables|Default|SetCursorPosition _location))
  (CallFunction|SetLocationonServer _output_get))

(event Custom|SetDataPlayer%20Multi
  (CallFunction|SetDataPlayers))

(event Custom|Set%20LocationOnServer
  (params (CursorPosition :type Vector))
  (Variables|Default|SetCursorPosition CursorPosition))

(event Custom|SetDataPlayers
  (bind _returnvalue (Game|GetGameState))
  (bind _playerarray (Variables|/Script/Engine.GameStateBase|GetPlayerArray _returnvalue))
  (bind _returnvalue_2 (Utilities|Array|Length _playerarray))
  (bind _returnvalue_3 (- _returnvalue_2 1))
  (bind _output_get (Variables|Default|SetPlayer%20Data (Utilities|Struct|MakeS_PlayerData _returnvalue_3 (Utilities|String|StringToName (Utilities|String|ToString(Text) (Utilities|Array|Get(acopy) (Variables|Default|GetArrayNamesPlayer) _returnvalue_3))) (Math|Conversions|ToLinearColor(Color) (Utilities|Array|Get(acopy) (Variables|Default|GetArrayColorsPlayer) _returnvalue_3)) "0.000000,0.000000,0.000000")))
  (CallFunction|SetDataPlayersonServer _output_get))

(event Custom|OtherCursors
  (params (CursorPosition :type Array%20of%20S%20Player%20Data%20Structures))
  (for _array_element CursorPosition
    (CallFunction|SetPlayersCursors _array_element)))

(event Custom|CreateCursor
  (bind _returnvalue (UserInterface|CreateWidget "/Game/00_Clase/UI/Cursores/WBP_DefaultCursor.WBP_DefaultCursor_C"))
  (bind _output_get (Variables|Default|SetWBP%20Cursor _returnvalue))
  (Class|PlayerController|SetMouseCursorWidget "Default" _output_get))

(event EventBeginPlay
  (Utilities|FlowControl|Sequence
    (:then_0
      (CallFunction|AddMappingContext))
    (:then_1
      (Input|SetInputModeGameandUI self 0 "DoNotLock" false false)
      (Variables|Default|SetbShowMouseCursor true))
    (:then_2
      (Class|WidgetBlueprintLibrary|SetFocustoGameViewport))
    (:then_3
      (Networking|SwitchHasAuthority
        (:Authority
          (CallFunction|SetDataPlayerMulti))))
    (:then_4
      (Utilities|Time|SetTimerbyEvent (EventDispatchers|CreateEvent :!event Custom|SaveCursorPosition) 0.1 true))
    (:then_5
      (CallFunction|CreateCursor))
    (:then_6
      (CallFunction|CreatePreviewBuildingBeginPlay "TOWNHALL"))))

(event Custom|UpdateSelectedElementUI
  (params (SelectedUIData :type S%20Selected%20UI%20Data%20Structure) (Actions :type Array%20of%20E_Actions%20Enums :default "NewEnumerator10") (Crafteables :type Map%20of%20Names%20to%20Booleans) (Queue :type Array%20of%20S%20Crafteable%20Structures))
  (Default|UpdateSelectedElementUI (CallFunction|GetHUDRef) SelectedUIData Actions Crafteables Queue))

(event Custom|RefreshResources
  (params (Resources :type Map%20of%20E_Resources%20Enums%20to%20Integers :default "NewEnumerator6"))
  (Default|RefreshResources (CallFunction|GetHUDRef) Resources))

(event Custom|RequestResourceUpdate
  (CallFunction|CalltoRefreshResourcesonServer))

(event Custom|CallToRefreshResourcesOnServer
  (bind _asps_rts (Utilities|Casting|CastToPS_RTS (Variables|GetPlayerState)))
  (Default|RefreshResourcesonServer _asps_rts))

(event Custom|RefreshUIProdTime
  (params (Time :type Float%20%28double-precision%29))
  (Default|RefreshUIProdTime (CallFunction|GetHUDRef) Time))

(event Custom|RemoveFromProduction
  (params (IndexToRemove :type Integer))
  (bind _selected_actor (Variables|/Game/00_Clase/Blueprints/Commons/PAWN_RTS.PAWN_RTS_C|GetSelected%20Actor (CallFunction|GetPawnRef))
    (:then
      (bind _asbp_base_definitive_building (Utilities|Casting|CastToBP_BaseDefinitiveBuilding _selected_actor))
      (Default|4-CancelProduction _asbp_base_definitive_building IndexToRemove))
    (:else)))

(event Custom|ConfirmBuilidingPreviewOnServer
  (params (Location :type Vector) (ID%20Building :type Name))
  (Default|SpawnBuildforPlayer (CallFunction|GetGSRef) self ID%20Building Location (.color (Variables|Default|GetPlayer%20Data))))

(event Custom|ConfirmBuildingLocation
  (params (ID%20Building :type Name) (Location :type Vector))
  (EventDispatchers|BindEventtoWorkingSiteCreated (CallFunction|GetGSRef) (EventDispatchers|CreateEvent :!event Custom|NewWorkingSiteCreated))
  (Default|CreateWorkingZone (CallFunction|GetGSRef) self ID%20Building Location))

(event Custom|ConfirmConstruction
  (bind _preview_building (Variables|Default|GetPreview%20Building)
    (:then
      (if (and (Default|CanIBuildHere _preview_building) (Default|CanIPayIt _preview_building))
        (CallFunction|ConfirmBuildingLocation (Variables|/Game/00_Clase/Blueprints/Buildings/BP_BaseBuilding.BP_BaseBuilding_C|GetID%20Selected%20Element _preview_building) (Transformation|GetActorLocation _preview_building))
        (Default|PaythePrice (Variables|Default|GetPreview%20Building))
        (CallFunction|CancelPreviewBuilding)
        (else
          (CallFunction|CantBuildHere))))
    (:else)))

(event Custom|Craft%20Something
  (params (ID%20Craft :type Name) (Price :type Map%20of%20E_Resources%20Enums%20to%20Integers :default "NewEnumerator6"))
  (if (Default|CanIPayIt (CallFunction|GetPSRef) Price)
    (bind _added (Default|OrdertoCraftSomething (CallFunction|GetPawnRef) ID%20Craft))
    (if _added
      (Default|AddRemoveResources (CallFunction|GetPSRef) Price false))
    (else
      (Development|PrintString "NO TIENES LOS RECURSOS SUFICENTES" true true "(R=1.000000,G=0.000000,B=0.000000,A=1.000000)"))))

(event Custom|ActionOrder
  (params (Action :type E_Actions%20Enum :default "NewEnumerator0"))
  (Default|GiveOrderfromPC (CallFunction|GetPawnRef) Action)
  (CallFunction|ActivateTargetMode Action))

(event Custom|Cant%20Build%20Here
  (Development|PrintString "NO SE PUEDE CONSTRUIR AQUI" true true "(R=1.000000,G=0.000000,B=0.000000,A=1.000000)"))

(event Custom|NewWorkingSiteCreated
  (params (Working%20Zone :type BP%20Working%20Zone%20Object%20Reference) (PC%20RTS :type PC%20RTS%20Object%20Reference))
  (if (== PC%20RTS self)
    (EventDispatchers|UnbindEventfromWorkingSiteCreated (CallFunction|GetGSRef) (delegate Custom|NewWorkingSiteCreated))
    (Default|NewBuildingCreated (CallFunction|GetPawnRef) Working%20Zone)))

(event Input|KeyboardEvents|NumPadOne
  (params (Key :type Key%20Structure))
  (:Pressed
    (CallFunction|CreatePreviewBuilding "BARRACKS")))

(event Input|KeyboardEvents|NumPadEight
  (params (Key :type Key%20Structure))
  (:Pressed
    (CallFunction|CreatePreviewBuilding "WATCH_TOWER")))

(event Input|KeyboardEvents|NumPadSeven
  (params (Key :type Key%20Structure))
  (:Pressed
    (CallFunction|CreatePreviewBuilding "TEMPLE")))

(event Input|KeyboardEvents|NumPadNine
  (params (Key :type Key%20Structure))
  (:Pressed
    (CallFunction|SpawnUnit "VILLAGER")))

(event Input|KeyboardEvents|NumPadTwo
  (params (Key :type Key%20Structure))
  (:Pressed
    (CallFunction|CreatePreviewBuilding "TOWNHALL")))

(event Input|KeyboardEvents|NumPadThree
  (params (Key :type Key%20Structure))
  (:Pressed
    (CallFunction|CreatePreviewBuilding "HOUSE")))

(event Input|KeyboardEvents|NumPadFour
  (params (Key :type Key%20Structure))
  (:Pressed
    (CallFunction|CreatePreviewBuilding "ARCHERY")))

(event Input|KeyboardEvents|NumPadFive
  (params (Key :type Key%20Structure))
  (:Pressed
    (CallFunction|CreatePreviewBuilding "PORT")))

(event Input|KeyboardEvents|NumPadSix
  (params (Key :type Key%20Structure))
  (:Pressed
    (CallFunction|CreatePreviewBuilding "STORAGE")))

(fn ConstructionScript)

(fn GetCursorPosition
  (params (TraceChannel :type ETraceTypeQuery%20Enum :default "TraceTypeQuery1"))
  (bind (_worldlocation _worlddirection) (Game|Player|ConvertMouseLocationToWorldSpace))
  (bind (_outhit _returnvalue) (Collision|LineTraceByChannel _worldlocation (+ _worldlocation (* _worlddirection 1e+07)) TraceChannel false 0 "None"))
  (if _returnvalue
    (return (.Location (Collision|BreakHitResult _outhit)))
    (else
      (return (Variables|Default|GetCursorPosition)))))

(fn GetHUDRef
  (Variables|Default|GetAs%20HUD%20RTS
    (:then
      _)
    (:else
      (bind _ashud_rts (Utilities|Casting|CastToHUD_RTS (HUD|GetHUD)))
      (Variables|Default|SetAs%20HUD%20RTS _ashud_rts)))
  (return (Variables|Default|GetAs%20HUD%20RTS)))

(fn GetGSRef
  (Variables|Default|GetAs%20GS%20RTS
    (:then
      _)
    (:else
      (bind _asgs_rts (Utilities|Casting|CastToGS_RTS (Game|GetGameState)))
      (Variables|Default|SetAs%20GS%20RTS _asgs_rts)))
  (return (Variables|Default|GetAs%20GS%20RTS)))

(fn GetPawnRef
  (Variables|Default|GetAs%20PAWN%20RTS
    (:then
      _)
    (:else
      (bind _aspawn_rts (Utilities|Casting|CastToPAWN_RTS (Game|Player|GetPlayerPawn 0)))
      (Variables|Default|SetAs%20PAWN%20RTS _aspawn_rts)))
  (return (Variables|Default|GetAs%20PAWN%20RTS)))

(fn SetPlayersCursors
  (params (S%20Player%20Data :type S%20Player%20Data%20Structure))
  (bind _cursors (Variables|Default|GetCursors))
  (bind (_value _returnvalue) (Utilities|Map|Find _cursors (.id S%20Player%20Data)))
  (if (not (== (.ID (Utilities|Struct|BreakS_PlayerData S%20Player%20Data)) (.ID (Utilities|Struct|BreakS_PlayerData (Variables|Default|GetPlayer%20Data)))))
    (if _returnvalue
      (Variables|/Game/00_Clase/Blueprints/Cursor/BP_Cursor.BP_Cursor_C|SetDestination%20Cursor%20Location _value (.cursorlocation S%20Player%20Data))
      (else
        (bind _returnvalue_2 (Game|SpawnActorfromClass "/Game/00_Clase/Blueprints/Cursor/BP_Cursor.BP_Cursor_C" (Math|Transform|MakeTransform (.cursorlocation S%20Player%20Data) "0, 0, 0" "1.000000,1.000000,1.000000") "Undefined" "MultiplyWithRoot" 0 S%20Player%20Data 0))
        (Utilities|Map|Add (Variables|Default|GetCursors) (.id S%20Player%20Data) _returnvalue_2)))))

(fn CancelPreviewBuilding
  (bind _preview_building (Variables|Default|GetPreview%20Building)
    (:then
      (Actor|DestroyActor _preview_building)
      (Variables|Default|SetPreview%20Building 0)
      (CallFunction|ActivateTargetMode "NewEnumerator10"))
    (:else)))

(fn GetPSRef
  (Variables|Default|GetAs%20PS%20RTS
    (:then
      _)
    (:else
      (bind _asps_rts (Utilities|Casting|CastToPS_RTS (Variables|GetPlayerState)))
      (Variables|Default|SetAs%20PS%20RTS _asps_rts)))
  (return (Variables|Default|GetAs%20PS%20RTS)))

(fn CreatePreviewBuilding
  (params (ID%20Selected%20Element :type Name))
  (Variables|Default|GetPreview%20Building
    (:then
      (CallFunction|CancelPreviewBuilding))
    (:else
      (bind _location (CallFunction|GetCursorPosition "TraceTypeQuery4"))
      (bind _returnvalue (Game|SpawnActorfromClass "/Game/00_Clase/Blueprints/Buildings/BP_BasePreviewBuilding.BP_BasePreviewBuilding_C" (Math|Transform|MakeTransform _location "0, 0, 0" "1.000000,1.000000,1.000000") "Undefined" "MultiplyWithRoot" self ID%20Selected%20Element (.color (Variables|Default|GetPlayer%20Data)) 0))
      (Variables|Default|SetPreview%20Building _returnvalue))))

(fn SpawnUnit
  (params (ID%20Selected%20Element :type Name))
  (bind _returnvalue (Utilities|GetDataTableRow "/Game/00_Clase/Blueprints/Structs/DT_Crafteable.DT_Crafteable" ID%20Selected%20Element)
    (:then
      (bind _output_get (LocalVariables|SetCrafteableData _returnvalue))
      (if (CallFunction|CanIPayIt (.Price (Utilities|Struct|BreakS_Crafteable _output_get)))
        (bind _location (CallFunction|GetCursorPosition "TraceTypeQuery4"))
        (Game|SpawnActorfromClass "/Game/00_Clase/Blueprints/Units/BP_BaseUnit.BP_BaseUnit_C" (Math|Transform|MakeTransform _location "0, 0, 0" "1.000000,1.000000,1.000000") "Undefined" "MultiplyWithRoot" self ID%20Selected%20Element "0.000000,0.000000,0.000000" 0)
        (Default|AddRemoveResources (CallFunction|GetPSRef) (.Price (Utilities|Struct|BreakS_Crafteable (LocalVariables|GetCrafteableData))) false)
        (else
          (Development|PrintString "RECURSOS INSUFICIENTES"))))))

(fn CanIPayIt
  (params (Price :type Map%20of%20E_Resources%20Enums%20to%20Integers :default "NewEnumerator6"))
  (bind _resources (Default|GetResourcesMap (CallFunction|GetPSRef)))
  (bind _keys (Utilities|Map|Keys Price))
  (for _array_element _keys
    (if (not (>= (.Value (Utilities|Map|Find _resources _array_element)) (.Value (Utilities|Map|Find Price _array_element))))
      (LocalVariables|SetNewLocalVar false)))
  (return (LocalVariables|GetNewLocalVar)))

(fn SpawnRallyPoint
  (bind _location (CallFunction|GetCursorPosition "TraceTypeQuery4"))
  (bind _returnvalue (Game|SpawnActorfromClass "/Game/00_Clase/Blueprints/Buildings/RallyPoint/BP_RallyPointPreview.BP_RallyPointPreview_C" (Math|Transform|MakeTransform _location "0, 0, 0" "1.000000,1.000000,1.000000") "Undefined" "MultiplyWithRoot" self 0))
  (Variables|Default|SetPreview%20Rally%20Point _returnvalue))

(fn CancelPreviewRallyPoint
  (bind _preview_rally_point (Variables|Default|GetPreview%20Rally%20Point)
    (:then
      (Actor|DestroyActor _preview_rally_point)
      (Variables|Default|SetPreview%20Rally%20Point 0))
    (:else)))

(fn ConfirmRallyPoint
  (bind _preview_rally_point (Variables|Default|GetPreview%20Rally%20Point)
    (:then
      (bind _selected_actor (Variables|/Game/00_Clase/Blueprints/Commons/PAWN_RTS.PAWN_RTS_C|GetSelected%20Actor (CallFunction|GetPawnRef))
        (:then
          (bind _asbp_base_definitive_building (Utilities|Casting|CastToBP_BaseDefinitiveBuilding _selected_actor))
          (Default|SpawnRallyPoint _asbp_base_definitive_building (Transformation|GetActorLocation _preview_rally_point))
          (CallFunction|CancelPreviewRallyPoint))
        (:else)))
    (:else)))

(fn ActivateTargetMode
  (params (Action :type E_Actions%20Enum :default "NewEnumerator10"))
  (Default|SetStatus (Variables|Default|GetWBP%20Cursor) Action))

(fn CreatePreviewBuildingBeginPlay
  (params (ID%20Selected%20Element :type Name))
  (bind _player_data (Variables|Default|GetPlayer%20Data))
  (Default|SpawnBuildforPlayer (CallFunction|GetGSRef) self ID%20Selected%20Element (Utilities|Array|Get(acopy) (Variables|Default|GetLocations) (.id _player_data)) (.color _player_data)))