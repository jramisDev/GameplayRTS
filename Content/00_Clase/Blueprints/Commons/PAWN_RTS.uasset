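; RTS player pawn that handles camera movement, pings, selection and orders.
; Zoom blends spring arm length and pitch with one alpha.
; Mouse traces drive clicks: left confirms building or rally-point placement or selects actors for the UI, right cancels placement or sends orders with a cursor effect.
; Server and multicast-named events handle pings, sounds and bounds-sized, player-colored selection decals, while a helper queues crafting in selected buildings.
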(event Custom|SpawnPingOnServer
  (params (PingType :type E_PingWorldType%20Enum :default "NewEnumerator0") (Spawn%20Transform%20Location :type Vector))
  (Game|SpawnActorfromClass "/Game/00_Clase/Blueprints/Pings/BP_Ping.BP_Ping_C" (Math|Transform|MakeTransform Spawn%20Transform%20Location "0, 0, 0" "1.000000,1.000000,1.000000") "Undefined" "MultiplyWithRoot" 0 PingType (Variables|/Game/00_Clase/Blueprints/Commons/PC_RTS.PC_RTS_C|GetPlayer%20Data (CallFunction|GetPCRef)) 0))

(event Custom|PlaySoundPingOnServer
  (params (Sound :type Object%20Soft%20Object%20Reference))
  (CallFunction|PlaySoundPingMulti Sound))

(event Custom|PlaySoundPingMulti
  (params (Asset :type Object%20Soft%20Object%20Reference))
  (bind _returnvalue (Utilities|LoadAssetBlocking Asset))
  (bind _assound_base (Utilities|Casting|CastToSoundBase _returnvalue))
  (Audio|PlaySound2D _assound_base 1.0 1.0 0.0 0 0))

(event Input|EnhancedActionEvents|EnhancedInputActionIA_Move
  (params (ActionValue :type Vector%202D%20Structure) (ElapsedSeconds :type Float%20%28double-precision%29) (TriggeredSeconds :type Float%20%28double-precision%29) (InputAction :type Input%20Action%20Object%20Reference :default "/Game/00_Clase/Input/IA_Move.IA_Move"))
  (Class|PawnMovementComponent|AddInputVector (Variables|Default|GetFloatingPawnMovement) (Math|Conversions|ToVector(Vector2D) ActionValue) false))

(event Input|EnhancedActionEvents|EnhancedInputActionIA_Ping
  (params (ActionValue :type Boolean) (ElapsedSeconds :type Float%20%28double-precision%29) (TriggeredSeconds :type Float%20%28double-precision%29) (InputAction :type Input%20Action%20Object%20Reference :default "/Game/00_Clase/Input/IA_Ping.IA_Ping"))
  (bind _as_pc_rts (CallFunction|GetPCRef))
  (bind _as_hud_rts (Default|GetHUDRef _as_pc_rts))
  (:Started
    (Default|ShowPingUI _as_hud_rts true))
  (:Completed
    (Default|ShowPingUI _as_hud_rts false)))

(event Input|EnhancedActionEvents|EnhancedInputActionIA_Ping1
  (params (ActionValue :type Boolean) (ElapsedSeconds :type Float%20%28double-precision%29) (TriggeredSeconds :type Float%20%28double-precision%29) (InputAction :type Input%20Action%20Object%20Reference :default "/Game/00_Clase/Input/IA_Ping1.IA_Ping1"))
  (:Started
    (CallFunction|SpawnPingonServer "NewEnumerator1" (CallFunction|PingPosition))))

(event Input|EnhancedActionEvents|EnhancedInputActionIA_Ping2
  (params (ActionValue :type Boolean) (ElapsedSeconds :type Float%20%28double-precision%29) (TriggeredSeconds :type Float%20%28double-precision%29) (InputAction :type Input%20Action%20Object%20Reference :default "/Game/00_Clase/Input/IA_Ping2.IA_Ping2"))
  (:Started
    (CallFunction|SpawnPingonServer "NewEnumerator4" (CallFunction|PingPosition))))

(event Input|EnhancedActionEvents|EnhancedInputActionIA_Zoom
  (params (ActionValue :type Float%20%28double-precision%29) (ElapsedSeconds :type Float%20%28double-precision%29) (TriggeredSeconds :type Float%20%28double-precision%29) (InputAction :type Input%20Action%20Object%20Reference :default "/Game/00_Clase/Input/IA_Zoom.IA_Zoom"))
  (bind _output_get (Variables|Default|SetAlpha (Math|Float|Clamp(Float) (+ (Variables|Default|GetAlpha) (/ ActionValue 1e+02)))))
  (Transformation|SetWorldRotation (Variables|Default|GetSpringArm) (Math|Rotator|MakeRotator 0.0 (Math|Float|Lerp (Variables|Camera|GetZoomAngleMax) (Variables|Camera|GetZoomAngleMin) _output_get) 0.0) false false)
  (Variables|/Script/Engine.SpringArmComponent|SetTargetArmLength (Variables|Default|GetSpringArm) (Math|Float|Lerp (Variables|Camera|GetHightMax) (Variables|Camera|GetHightMin) _output_get)))

(event Custom|AddDecalEffectMulticast
  (params (Target :type Actor%20Object%20Reference) (Color :type Linear%20Color%20Structure))
  (bind _boxextent (Collision|GetActorBounds Target true false))
  (bind (_x _y) (Math|Vector|BreakVector _boxextent))
  (bind _returnvalue (> _y _x))
  (bind _returnvalue_2 (select _returnvalue _y _x))
  (bind _returnvalue_3 (/ _returnvalue_2 5e+01))
  (bind _returnvalue_4 (AddComponent|AddDecalComponent Target false (Math|Transform|MakeTransform "0, 0, 0" "90.000000,0.000000,0.000000" (Math|Vector|MakeVector 1.0 _returnvalue_3 _returnvalue_3))))
  (bind _returnvalue_5 (Rendering|Material|CreateDynamicMaterialInstance "/Game/00_Clase/Materials/Decals/M_Selected.M_Selected" "None" "None" :!class /Script/Engine.KismetMaterialLibrary))
  (Rendering|Material|SetVectorParameterValue _returnvalue_5 "Color" Color :!class /Script/Engine.MaterialInstanceDynamic)
  (Rendering|Components|Decal|SetDecalMaterial _returnvalue_4 _returnvalue_5))

(event Custom|RemoveSelectDecalOnServer
  (params (Target :type Object%20Object%20Reference))
  (CallFunction|RemoveElementMulti Target))

(event Custom|RemoveElementMulti
  (params (Target :type Object%20Object%20Reference))
  (Class|BPISelectable|Deselect(Message) Target))

(event Custom|SelectElementOnServer
  (params (Target :type Actor%20Object%20Reference) (PC :type PC%20RTS%20Object%20Reference))
  (CallFunction|AddDecalEffectMulticast Target (.color (Variables|/Game/00_Clase/Blueprints/Commons/PC_RTS.PC_RTS_C|GetPlayer%20Data PC))))

(event Input|EnhancedActionEvents|EnhancedInputActionIA_LeftClick
  (params (ActionValue :type Boolean) (ElapsedSeconds :type Float%20%28double-precision%29) (TriggeredSeconds :type Float%20%28double-precision%29) (InputAction :type Input%20Action%20Object%20Reference :default "/Game/00_Clase/Input/IA_LeftClick.IA_LeftClick"))
  (bind _as_pc_rts (CallFunction|GetPCRef))
  (bind _as_pc_rts_2 (CallFunction|GetPCRef))
  (bind _as_pc_rts_3 (CallFunction|GetPCRef))
  (bind (_worldlocation _worlddirection) (Game|Player|ConvertMouseLocationToWorldSpace _as_pc_rts_2))
  (:Started
    (Variables|/Game/00_Clase/Blueprints/Commons/PC_RTS.PC_RTS_C|GetPreview%20Building _as_pc_rts_3
      (:then
        (Default|ConfirmConstruction _as_pc_rts_3))
      (:else
        (Variables|/Game/00_Clase/Blueprints/Commons/PC_RTS.PC_RTS_C|GetPreview%20Rally%20Point _as_pc_rts
          (:then
            (Default|ConfirmRallyPoint _as_pc_rts))
          (:else
            (bind (_outhit _returnvalue) (Collision|LineTraceByChannel _worldlocation (+ _worldlocation (* _worlddirection 1e+06)) "TraceTypeQuery3" false 0 "None"))
            (if _returnvalue
              (bind _selected_actor (Variables|Default|GetSelected%20Actor)
                (:then
                  (Class|BPISelectable|Deselect(Message) _selected_actor)
                  (CallFunction|RemoveSelectDecalonServer _selected_actor)
                  (Variables|Default|SetSelected%20Actor 0))
                (:else
                  _))
              (bind _output_get (Variables|Default|SetSelected%20Actor (.HitActor (Collision|BreakHitResult _outhit))))
              (bind (_ui_data _actions _crafteables _queue) (Class|BPISelectable|Selected(Message) _output_get))
              (Default|UpdateSelectedElementUI (CallFunction|GetPCRef) _ui_data _actions _crafteables _queue)
              (CallFunction|SelectElementonServer (Variables|Default|GetSelected%20Actor) (CallFunction|GetPCRef))
              (else
                (bind _selected_actor_2 (Variables|Default|GetSelected%20Actor)
                  (:then
                    (Class|BPISelectable|Deselect(Message) _selected_actor_2)
                    (CallFunction|RemoveSelectDecalonServer _selected_actor_2)
                    (Variables|Default|SetSelected%20Actor 0)
                    (Default|UpdateSelectedElementUI :self (CallFunction|GetPCRef) :Actions "NewEnumerator0" :Crafteables (Utilities|Map|MakeMap "None" false)))
                  (:else))))))))))

(event Custom|SpawnNiagaraCursor
  (params (Spawn%20Transform%20Location :type Vector))
  (bind _as_pc_rts (CallFunction|GetPCRef))
  (bind _player_data (Variables|/Game/00_Clase/Blueprints/Commons/PC_RTS.PC_RTS_C|GetPlayer%20Data _as_pc_rts))
  (Game|SpawnActorfromClass "/Game/00_Clase/Blueprints/Cursor/BP_FeedbackCursor.BP_FeedbackCursor_C" (Math|Transform|MakeTransform Spawn%20Transform%20Location "0, 0, 0" "1.000000,1.000000,1.000000") "Undefined" "MultiplyWithRoot" 0 (Utilities|Text|ToText(Name) (.name _player_data)) (Math|Conversions|ToColor(LinearColor) (.color _player_data)) 0))

(event Custom|GiveOrderToAIC
  (params (Actor :type Actor%20Object%20Reference) (Order :type E_Actions%20Enum :default "NewEnumerator0") (TargetLocation :type Vector) (TargetActor :type Actor%20Object%20Reference))
  (Class|BPIOrders|GiveGenericOrder(Message) Actor Order TargetLocation TargetActor "None"))

(event Input|EnhancedActionEvents|EnhancedInputActionIA_RightClick
  (params (ActionValue :type Boolean) (ElapsedSeconds :type Float%20%28double-precision%29) (TriggeredSeconds :type Float%20%28double-precision%29) (InputAction :type Input%20Action%20Object%20Reference :default "/Game/00_Clase/Input/IA_RightClick.IA_RightClick"))
  (bind _as_pc_rts (CallFunction|GetPCRef))
  (bind _as_pc_rts_2 (CallFunction|GetPCRef))
  (bind (_worldlocation _worlddirection) (Game|Player|ConvertMouseLocationToWorldSpace _as_pc_rts))
  (:Started
    (Variables|/Game/00_Clase/Blueprints/Commons/PC_RTS.PC_RTS_C|GetPreview%20Building _as_pc_rts_2
      (:then
        (Default|CancelPreviewBuilding (CallFunction|GetPCRef)))
      (:else
        (Variables|/Game/00_Clase/Blueprints/Commons/PC_RTS.PC_RTS_C|GetPreview%20Rally%20Point _as_pc_rts_2
          (:then
            (Default|CancelPreviewRallyPoint (CallFunction|GetPCRef)))
          (:else
            (bind (_outhit _returnvalue) (Collision|LineTraceByChannel _worldlocation (+ _worldlocation (* _worlddirection 1e+06)) "TraceTypeQuery1" false 0 "None"))
            (if _returnvalue
              (CallFunction|SpawnNiagaraCursor (.Location (Collision|BreakHitResult _outhit)))
              (CallFunction|GiveOrdertoSelectedActor (.Location (Collision|BreakHitResult _outhit)) (.HitActor (Collision|BreakHitResult _outhit)))
              (else
                (bind _selected_actor (Variables|Default|GetSelected%20Actor)
                  (:then
                    (CallFunction|GiveOrdertoAIC _selected_actor "NewEnumerator1" "0, 0, 0"))
                  (:else))))))))))

(fn ConstructionScript)

(fn GetPCRef
  (Variables|Default|GetAs%20PC%20RTS
    (:then
      _)
    (:else
      (bind _aspc_rts (Utilities|Casting|CastToPC_RTS (Components|GetOwner)))
      (Variables|Default|SetAs%20PC%20RTS _aspc_rts)))
  (return (Variables|Default|GetAs%20PC%20RTS)))

(fn SetZoomItOut
  (params (A :type Float%20%28double-precision%29))
  (Variables|/Script/Engine.SpringArmComponent|SetTargetArmLength (Variables|Default|GetSpringArm) (Math|Interpolation|FInterpTo (Variables|/Script/Engine.SpringArmComponent|GetTargetArmLength (Variables|Default|GetSpringArm)) (Math|Float|Clamp(Float) (+ (* A (Variables|Camera|GetSensitivityZoom)) (Variables|/Script/Engine.SpringArmComponent|GetTargetArmLength (Variables|Default|GetSpringArm))) (Variables|Camera|GetHightMin) (Variables|Camera|GetHightMax)) 5.0 1.0)))

(fn SetRotationZoom
  (bind _springarm (Variables|Default|GetSpringArm))
  (bind _returnvalue (Transformation|GetWorldRotation _springarm))
  (Transformation|SetWorldRotation (Variables|Default|GetSpringArm) (Math|Rotator|MakeRotator (.roll _returnvalue) (Math|Float|MapRangeClamped (Variables|/Script/Engine.SpringArmComponent|GetTargetArmLength (Variables|Default|GetSpringArm)) (Variables|Camera|GetHightMin) (Variables|Camera|GetHightMax) (Variables|Camera|GetZoomAngleMax) (Variables|Camera|GetZoomAngleMin)) (.yaw _returnvalue)) false false))

(fn PingPosition
  (bind _as_pc_rts (CallFunction|GetPCRef))
  (bind (_worldlocation _worlddirection) (Game|Player|ConvertMouseLocationToWorldSpace _as_pc_rts))
  (bind (_outhit _returnvalue) (Collision|LineTraceByChannel _worldlocation (+ _worldlocation (* _worlddirection 1e+06)) "TraceTypeQuery1" false 0 "None"))
  (if _returnvalue
    _
    (else
      _))
  (return (.Location (Collision|BreakHitResult _outhit))))

(fn OrdertoCraftSomething
  (params (ID%20Craft :type Name))
  (bind _selected_actor (Variables|Default|GetSelected%20Actor)
    (:then
      (bind _asbp_base_definitive_building (Utilities|Casting|CastToBP_BaseDefinitiveBuilding _selected_actor))
      (if (Default|DoIHaveSpaceinProduction _asbp_base_definitive_building)
        (Default|1-AddItemtoQueue _asbp_base_definitive_building ID%20Craft))
      (return (Default|DoIHaveSpaceinProduction _asbp_base_definitive_building)))
    (:else)))

(fn GiveOrdertoSelectedActor
  (params (Location :type Vector) (ActorOrder :type Actor%20Object%20Reference))
  (bind _selected_actor (Variables|Default|GetSelected%20Actor)
    (:then
      (CallFunction|GiveOrdertoAIC _selected_actor "NewEnumerator10" Location ActorOrder))
    (:else)))