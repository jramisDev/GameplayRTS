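; HUD for the RTS player that creates the main UI and acts as the bridge between its widgets and PC_RTS.
; It pushes selection details, actions, craftables, resources and production timing into sub-widgets, and forwards craft, queue-removal and action orders to the controller.
; It also creates and removes the selection-ping and hover-info widgets, relays ping sounds to PAWN_RTS, and lazily caches controller and pawn references.
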(event Custom|UpdateSelectedElementUI
  (params (SelectedUIData :type S%20Selected%20UI%20Data%20Structure) (Actions :type Array%20of%20E_Actions%20Enums :default "NewEnumerator10") (Crafteables :type Map%20of%20Names%20to%20Booleans) (Queue :type Array%20of%20S%20Crafteable%20Structures))
  (bind _wbp_main_ui (Variables|Default|GetWBP%20Main%20UI)
    (:then
      (Default|SetData (Variables|/Game/00_Clase/UI/HUD/WBP_MainUI.WBP_MainUI_C|GetWBP_SelectedDetails _wbp_main_ui) SelectedUIData Queue)
      (Default|SetActions (Variables|/Game/00_Clase/UI/HUD/WBP_MainUI.WBP_MainUI_C|GetWBP_Actions _wbp_main_ui) Actions Crafteables))
    (:else)))

(event Custom|ShowPingUI
  (params (OnOff :type Boolean))
  (CallFunction|ToggleWidgetPing OnOff))

(event Custom|Craft%20Element
  (params (ID%20Craft :type Name) (Price :type Map%20of%20E_Resources%20Enums%20to%20Integers :default "NewEnumerator6"))
  (Default|CraftSomething (CallFunction|GetPCRef) ID%20Craft Price))

(event Custom|RefreshResources
  (params (Resources :type Map%20of%20E_Resources%20Enums%20to%20Integers :default "NewEnumerator6"))
  (bind _wbp_main_ui (Variables|Default|GetWBP%20Main%20UI)
    (:then
      (Default|UpdateResources (Variables|/Game/00_Clase/UI/HUD/WBP_MainUI.WBP_MainUI_C|GetWBP_Resources _wbp_main_ui) Resources))
    (:else)))

(event Custom|RefreshUIProdTime
  (params (Time :type Float%20%28double-precision%29))
  (bind _wbp_main_ui (Variables|Default|GetWBP%20Main%20UI)
    (:then
      (Default|StartProduction (Variables|/Game/00_Clase/UI/HUD/WBP_SelectedDetails.WBP_SelectedDetails_C|GetWBP_Queue (Variables|/Game/00_Clase/UI/HUD/WBP_MainUI.WBP_MainUI_C|GetWBP_SelectedDetails _wbp_main_ui)) Time))
    (:else)))

(event Custom|RemoveFromProduction
  (params (IndexToRemove :type Integer))
  (Default|RemovefromProduction (CallFunction|GetPCRef) IndexToRemove))

(event Custom|SendActionOrderToPC
  (params (Action :type E_Actions%20Enum :default "NewEnumerator0"))
  (Default|ActionOrder (CallFunction|GetPCRef) Action))

(event EventBeginPlay
  (bind _returnvalue (UserInterface|CreateWidget "/Game/00_Clase/UI/HUD/WBP_MainUI.WBP_MainUI_C"))
  (bind _output_get (Variables|Default|SetWBP%20Main%20UI _returnvalue))
  (UserInterface|Viewport|AddtoViewport _output_get 0)
  (Default|RequestResourceUpdate (CallFunction|GetPCRef)))

(fn ConstructionScript)

(fn ToggleWidgetPing
  (params (Condition :type Boolean))
  (if Condition
    (Variables|Default|GetWBP_SelectionPing
      (:then)
      (:else
        (bind _returnvalue (UserInterface|CreateWidget "/Game/00_Clase/UI/Pings/WBP_SelectionPing.WBP_SelectionPing_C"))
        (bind _output_get (Variables|Default|SetWBP_SelectionPing _returnvalue))
        (UserInterface|Viewport|AddtoViewport _output_get 0)
        (EventDispatchers|BindEventtoSpawnPing _returnvalue (EventDispatchers|CreateEvent :!event PlaySoundinPawn))))
    (else
      (bind _wbp_selectionping (Variables|Default|GetWBP_SelectionPing)
        (:then
          (Widget|RemovefromParent _wbp_selectionping)
          (Variables|Default|SetWBP_SelectionPing 0))
        (:else)))))

(fn PlaySoundinPawn
  (params (Sound :type Sound%20Base%20Soft%20Object%20Reference))
  (Default|PlaySoundPingonServer (CallFunction|GetPCPawn) Sound))

(fn GetPCPawn
  (Variables|Default|GetAs%20PAWN%20RTS
    (:then
      _)
    (:else
      (bind _aspawn_rts (Utilities|Casting|CastToPAWN_RTS (Class|HUD|GetOwningPawn)))
      (Variables|Default|SetAs%20PAWN%20RTS _aspawn_rts)))
  (return (Variables|Default|GetAs%20PAWN%20RTS)))

(fn GetPCRef
  (Variables|Default|GetAs%20PC%20RTS
    (:then
      _)
    (:else
      (bind _aspc_rts (Utilities|Casting|CastToPC_RTS (Game|Player|GetOwningPlayerController)))
      (Variables|Default|SetAs%20PC%20RTS _aspc_rts)))
  (return (Variables|Default|GetAs%20PC%20RTS)))

(fn CreateHoverInfoWindow
  (params (Name :type Text) (Description :type Text) (Time :type Float%20%28double-precision%29) (Price :type Map%20of%20E_Resources%20Enums%20to%20Integers :default "NewEnumerator6"))
  (Variables|Default|GetWBP%20HoverInfo
    (:then)
    (:else
      (CallFunction|CloseHoverInfo)
      (bind _returnvalue (UserInterface|CreateWidget "/Game/00_Clase/UI/HUD/ActionsDetails/_WBP_HoverInfo._WBP_HoverInfo_C" 0 Name Description Time Price))
      (bind _output_get (Variables|Default|SetWBP%20HoverInfo _returnvalue))
      (bind _wbp_main_ui (Variables|Default|GetWBP%20Main%20UI)
        (:then
          (bind _returnvalue_2 (Class|CanvasPanel|AddChildtoCanvas (Variables|/Game/00_Clase/UI/HUD/WBP_MainUI.WBP_MainUI_C|GetCanvasPanel_34 _wbp_main_ui) _output_get))
          (Class|CanvasPanelSlot|SetAnchors _returnvalue_2 (Utilities|Struct|MakeAnchors "(X=0.810000,Y=0.300000)" "(X=1.000000,Y=0.770000)"))
          (Class|CanvasPanelSlot|SetOffsets _returnvalue_2))
        (:else)))))

(fn CloseHoverInfo
  (bind _wbp_hoverinfo (Variables|Default|GetWBP%20HoverInfo)
    (:then
      (Widget|RemovefromParent _wbp_hoverinfo)
      (Variables|Default|SetWBP%20HoverInfo 0))
    (:else)))