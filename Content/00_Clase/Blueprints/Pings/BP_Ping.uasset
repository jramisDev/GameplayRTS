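; Short-lived world ping actor that shows the player's name in their color, a ping type label and a Niagara effect, and plays a 2D sound.
; On BeginPlay it looks up DT_PingWorld by PingType and routes HERE or DEFIENDE to PingHere or PingDefense.
; Both functions are identical, tinting text and effect from the row and loading its Niagara and sound assets with blocking loads.
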(event EventBeginPlay
  (bind _txt_playername (Variables|Default|GetTXT_PlayerName))
  (bind _dataplayer (Variables|Default|GetDataPlayer))
  (Actor|SetLifeSpan 1.0)
  (Rendering|Components|TextRender|SetText _txt_playername (Utilities|Text|ToText(Name) (.name _dataplayer)))
  (Rendering|Components|TextRender|SetTextRenderColor _txt_playername (Math|Conversions|ToColor(LinearColor) (.color _dataplayer)))
  (bind _returnvalue (Utilities|GetDataTableRow "/Game/00_Clase/Blueprints/Structs/DT_PingWorld.DT_PingWorld" (Utilities|String|StringToName (Utilities|String|EnumtoString (Variables|Default|GetPingType))))
    (:then
      (switch Utilities|FlowControl|Switch|SwitchonE_PingWorldType (Variables|Default|GetPingType)
        (:NewEnumerator1
          (CallFunction|PingHere _returnvalue))
        (:NewEnumerator4
          (CallFunction|PingDefense _returnvalue))))))

(fn ConstructionScript)

(fn PingHere
  (params (S%20Ping :type S%20Pings%20World%20Structure))
  (bind (_type _niagara _sound _color) (Utilities|Struct|BreakS_PingsWorld S%20Ping))
  (bind _txt_ping (Variables|Default|GetTXT_Ping))
  (Rendering|Components|TextRender|SetText _txt_ping (Utilities|Text|ToText(String) (Utilities|String|EnumtoString _type)))
  (Rendering|Components|TextRender|SetTextRenderColor _txt_ping _color)
  (bind _returnvalue (Utilities|LoadAssetBlocking _niagara))
  (bind _asniagara_system (Utilities|Casting|CastToNiagaraSystem _returnvalue))
  (Class|NiagaraComponent|SetAsset (Variables|Default|GetNiagara) _asniagara_system true)
  (Niagara|SetNiagaraVariable(LinearColor) (Variables|Default|GetNiagara) "Color" (Math|Conversions|ToLinearColor(Color) _color))
  (bind _returnvalue_2 (Utilities|LoadAssetBlocking _sound))
  (bind _assound_base (Utilities|Casting|CastToSoundBase _returnvalue_2))
  (Audio|PlaySound2D _assound_base 1.0 1.0 0.0 0 0))

(fn PingDefense
  (params (S%20Ping :type S%20Pings%20World%20Structure))
  (bind (_type _niagara _sound _color) (Utilities|Struct|BreakS_PingsWorld S%20Ping))
  (bind _txt_ping (Variables|Default|GetTXT_Ping))
  (Rendering|Components|TextRender|SetText _txt_ping (Utilities|Text|ToText(String) (Utilities|String|EnumtoString _type)))
  (Rendering|Components|TextRender|SetTextRenderColor _txt_ping _color)
  (bind _returnvalue (Utilities|LoadAssetBlocking _niagara))
  (bind _asniagara_system (Utilities|Casting|CastToNiagaraSystem _returnvalue))
  (Class|NiagaraComponent|SetAsset (Variables|Default|GetNiagara) _asniagara_system true)
  (Niagara|SetNiagaraVariable(LinearColor) (Variables|Default|GetNiagara) "Color" (Math|Conversions|ToLinearColor(Color) _color))
  (bind _returnvalue_2 (Utilities|LoadAssetBlocking _sound))
  (bind _assound_base (Utilities|Casting|CastToSoundBase _returnvalue_2))
  (Audio|PlaySound2D _assound_base 1.0 1.0 0.0 0 0))