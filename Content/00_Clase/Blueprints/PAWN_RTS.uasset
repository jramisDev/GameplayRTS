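; RTS player pawn that acts as the camera rig, with Enhanced Input panning through FloatingPawnMovement and zooming by shifting the camera's world height.
; Mouse clicks line-trace from the deprojected cursor: left click prints and debug-draws the hit, right click spawns a BP_FeedbackCursor there.
; A lazily cached PC_RTS owner reference supplies the deprojection and the player name and color passed to the cursor.
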(event Custom|SpawnNiagaraCursor
  (params (Spawn%20Transform%20Location :type Vector))
  (bind _as_pc_rts (CallFunction|GetPCRef))
  (Game|SpawnActorfromClass "/Game/00_Clase/Blueprints/Cursor/BP_FeedbackCursor.BP_FeedbackCursor_C" (Math|Transform|MakeTransform Spawn%20Transform%20Location "0, 0, 0" "1.000000,1.000000,1.000000") "Undefined" "MultiplyWithRoot" 0 (Variables|/Game/00_Clase/Blueprints/PC_RTS.PC_RTS_C|GetNamePlayer _as_pc_rts) (Variables|/Game/00_Clase/Blueprints/PC_RTS.PC_RTS_C|GetColorPlayer _as_pc_rts) 0))

(event Input|EnhancedActionEvents|EnhancedInputActionIA_Move
  (params (ActionValue :type Vector%202D%20Structure) (ElapsedSeconds :type Float%20%28double-precision%29) (TriggeredSeconds :type Float%20%28double-precision%29) (InputAction :type Input%20Action%20Object%20Reference :default "/Game/00_Clase/Input/IA_Move.IA_Move"))
  (Class|PawnMovementComponent|AddInputVector (Variables|Default|GetFloatingPawnMovement) (Math|Conversions|ToVector(Vector2D) ActionValue) false))

(event Input|EnhancedActionEvents|EnhancedInputActionIA_Zoom
  (params (ActionValue :type Float%20%28double-precision%29) (ElapsedSeconds :type Float%20%28double-precision%29) (TriggeredSeconds :type Float%20%28double-precision%29) (InputAction :type Input%20Action%20Object%20Reference :default "/Game/00_Clase/Input/IA_Zoom.IA_Zoom"))
  (Transformation|AddWorldOffset (Variables|Default|GetCamera) (Math|Vector|MakeVector 0.0 0.0 (* ActionValue (Variables|Default|GetSensitivityZoom))) false false))

(event Input|EnhancedActionEvents|EnhancedInputActionIA_LeftClick
  (params (ActionValue :type Boolean) (ElapsedSeconds :type Float%20%28double-precision%29) (TriggeredSeconds :type Float%20%28double-precision%29) (InputAction :type Input%20Action%20Object%20Reference :default "/Game/00_Clase/Input/IA_LeftClick.IA_LeftClick"))
  (bind _as_pc_rts (CallFunction|GetPCRef))
  (bind (_worldlocation _worlddirection) (Game|Player|ConvertMouseLocationToWorldSpace _as_pc_rts))
  (:Started
    (bind (_outhit _returnvalue) (Collision|LineTraceByChannel _worldlocation (+ _worldlocation (* _worlddirection 1e+06)) "TraceTypeQuery1" false 0 "None"))
    (if _returnvalue
      (Development|PrintString (Utilities|GetDisplayName (.HitActor (Collision|BreakHitResult _outhit))))
      (Rendering|Debug|DrawDebugSphere (.Location (Collision|BreakHitResult _outhit)) 25.0 12 "(R=1.000000,G=1.000000,B=0.000000,A=1.000000)" 3.0))))

(event Input|EnhancedActionEvents|EnhancedInputActionIA_RightClick
  (params (ActionValue :type Boolean) (ElapsedSeconds :type Float%20%28double-precision%29) (TriggeredSeconds :type Float%20%28double-precision%29) (InputAction :type Input%20Action%20Object%20Reference :default "/Game/00_Clase/Input/IA_RightClick.IA_RightClick"))
  (bind _as_pc_rts (CallFunction|GetPCRef))
  (bind (_worldlocation _worlddirection) (Game|Player|ConvertMouseLocationToWorldSpace _as_pc_rts))
  (:Started
    (bind (_outhit _returnvalue) (Collision|LineTraceByChannel _worldlocation (+ _worldlocation (* _worlddirection 1e+06)) "TraceTypeQuery1" false 0 "None"))
    (if _returnvalue
      (CallFunction|SpawnNiagaraCursor (.Location (Collision|BreakHitResult _outhit))))))

(fn ConstructionScript)

(fn GetPCRef
  (Variables|Default|GetAs%20PC%20RTS
    (:then
      _)
    (:else
      (bind _aspc_rts (Utilities|Casting|CastToPC_RTS (Components|GetOwner)))
      (Variables|Default|SetAs%20PC%20RTS _aspc_rts)))
  (return (Variables|Default|GetAs%20PC%20RTS)))