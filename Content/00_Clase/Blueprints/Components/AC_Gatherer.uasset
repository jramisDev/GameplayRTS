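; AC_Gatherer is an actor component that gives its owner a single-type resource backpack for gathering.
; Adding resources stacks the same type, while a different type replaces the current contents.
; Gathering damage is capped by remaining space when the type matches, and otherwise uses the full damage value.
; Emptying returns the stored amount and type, then resets the amount to zero.
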(event EventBeginPlay)

(event EventTick
  (params (DeltaSeconds :type Float%20%28single-precision%29)))

(fn AddQuantitytoBackpack
  (params (Quantity%20to%20Add :type Integer) (Resource%20Type :type E_Resources%20Enum :default "NewEnumerator6"))
  (if (<= (Variables|Default|GetBackpackSizeCurrent) 0)
    (Variables|Default|SetResourceTypeOnBackpack Resource%20Type)
    (Variables|Default|SetBackpackSizeCurrent (+ (Variables|Default|GetBackpackSizeCurrent) Quantity%20to%20Add) :!label _label)
    (elif (Utilities|Enum|Equal(Enum) Resource%20Type (Variables|Default|GetResourceTypeOnBackpack))
      (goto _label)
      (else
        (Variables|Default|SetResourceTypeOnBackpack Resource%20Type)
        (Variables|Default|SetBackpackSizeCurrent Quantity%20to%20Add)))))

(fn EmptyBackpack
  (LocalVariables|SetNewLocalVar (Variables|Default|GetBackpackSizeCurrent))
  (Variables|Default|SetBackpackSizeCurrent 0)
  (return (LocalVariables|GetNewLocalVar) (Variables|Default|GetResourceTypeOnBackpack)))

(fn GetDamagetoResource
  (params (Type :type E_Resources%20Enum :default "NewEnumerator6"))
  (bind _returnvalue (CallFunction|GetRemainingBackpackSize))
  (if (Utilities|Enum|Equal(Enum) Type (Variables|Default|GetResourceTypeOnBackpack))
    (return (select (< _returnvalue (Variables|Default|GetDamageToResource)) _returnvalue (Variables|Default|GetDamageToResource)))
    (else
      (return (Variables|Default|GetDamageToResource)))))

(fn GetCurrentQuantity
  (return (Variables|Default|GetResourceTypeOnBackpack) (Variables|Default|GetBackpackSizeCurrent)))

(fn GetRemainingBackpackSize
  (return (- (Variables|Default|GetBackpackSizeMax) (Variables|Default|GetBackpackSizeCurrent))))