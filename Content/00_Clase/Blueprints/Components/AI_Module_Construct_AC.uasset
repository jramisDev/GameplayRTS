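; AI order module component that lets a unit construct a BP_WorkingZone building site.
; DoYourAction compares the unit's distance to the zone against its building size; in range, it increases working progress and starts a short timer.
; Out of range, it issues two orders on the zone through the AI controller, likely move then construct, and completes.
; StartOver, apparently the timer callback, re-issues the construct order and completes, forming a repeating work loop through the order system.
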(event Custom|StartOver
  (Default|GiveOrdertoActor (CallFunction|GetAIC) "NewEnumerator3" (Variables|Default|GetAs%20BP%20Working%20Zone))
  (Default|CallDoneOrder))

(event EventBeginPlay
  (|CallParentFunction) ; This node is disabled and will not be called.\nDrag off pins to build functionality.
)

(event EventTick
  (params (DeltaSeconds :type Float%20%28single-precision%29))
  (|CallParentFunction DeltaSeconds) ; This node is disabled and will not be called.\nDrag off pins to build functionality.
)

(fn DoYourAction
  (params (Location :type Vector :default "0, 0, 0") (Actor :type Actor%20Object%20Reference) (Id :type Name :default "None"))
  (|CallParentFunction Location Actor Id)
  (bind _asbp_working_zone (Utilities|Casting|CastToBP_WorkingZone (Variables|Default|GetActor)))
  (Variables|Default|SetAs%20BP%20Working%20Zone _asbp_working_zone)
  (if (CallFunction|CheckDistanceBetweenUnitBuild)
    (Default|IncreaseWorkingProgress (Variables|Default|GetAs%20BP%20Working%20Zone))
    (Utilities|Time|SetTimerbyEvent (EventDispatchers|CreateEvent :!event Custom|StartOver) 0.2)
    (else
      (Default|GiveOrdertoActor (CallFunction|GetAIC) "NewEnumerator0" (Variables|Default|GetAs%20BP%20Working%20Zone))
      (Default|GiveOrdertoActor (CallFunction|GetAIC) "NewEnumerator3" (Variables|Default|GetAs%20BP%20Working%20Zone))
      (Default|CallDoneOrder))))

(fn IsValidforOrder
  (params (Location :type Vector :default "0, 0, 0") (Actor :type Actor%20Object%20Reference) (Id :type Name :default "None"))
  (|CallParentFunction Location Actor Id)
  (return (and (== (Utilities|GetClass Actor) "/Game/00_Clase/Blueprints/Buildings/BP_WorkingZone.BP_WorkingZone_C") (Utilities|IsValid Actor))))

(fn CheckDistanceBetweenUnitBuild
  (bind _as_bp_working_zone (Variables|Default|GetAs%20BP%20Working%20Zone))
  (return (<= (Math|Vector|Distance(Vector) (Transformation|GetActorLocation _as_bp_working_zone) (Transformation|GetActorLocation (Default|GetUnitRef (CallFunction|GetAIC)))) (* (.x (Variables|/Game/00_Clase/Blueprints/Buildings/BP_WorkingZone.BP_WorkingZone_C|GetBuilding%20Size _as_bp_working_zone)) 1e+02))))