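; AI_Module_AC is a base actor component for AI behavior modules owned by an AIC_UnitBase controller.
; IsValidForOrder receives a location, actor and ID but returns false, and DoYourAction is empty, so both act as stubs, apparently for child modules to override.
; GetAIC lazily casts the owner to AIC_UnitBase and caches the reference for later calls.
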(event EventBeginPlay)

(event EventTick
  (params (DeltaSeconds :type Float%20%28single-precision%29)))

(fn IsValidforOrder
  (params (Location :type Vector) (Actor :type Actor%20Object%20Reference) (Id :type Name))
  (Variables|Default|SetLocation Location)
  (Variables|Default|SetActor Actor)
  (Variables|Default|SetId Id)
  (return false))

(fn GetAIC
  (Variables|Default|GetAs%20AIC%20Unit%20Base
    (:then
      _)
    (:else
      (bind _asaic_unit_base (Utilities|Casting|CastToAIC_UnitBase (Components|GetOwner)))
      (Variables|Default|SetAs%20AIC%20Unit%20Base _asaic_unit_base)))
  (return (Variables|Default|GetAs%20AIC%20Unit%20Base)))

(fn DoYourAction)