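; AI module component that handles the stop order for an AI-controlled unit.
; It accepts an order only when there is no valid location, no valid actor and the Id is "none".
; Its action calls the parent implementation, then immediately halts the unit's CharacterMovement through the AI controller's unit reference.
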(event EventBeginPlay
  (|CallParentFunction) ; This node is disabled and will not be called.\nDrag off pins to build functionality.
)

(event EventTick
  (params (DeltaSeconds :type Float%20%28single-precision%29))
  (|CallParentFunction DeltaSeconds) ; This node is disabled and will not be called.\nDrag off pins to build functionality.
)

(fn DoYourAction
  (|CallParentFunction)
  (Components|Movement|StopMovementImmediately (Variables|/Script/Engine.Character|GetCharacterMovement (Default|GetUnitRef (CallFunction|GetAIC)))))

(fn IsValidforOrder
  (params (Location :type Vector :default "0, 0, 0") (Actor :type Actor%20Object%20Reference) (Id :type Name :default "None"))
  (|CallParentFunction Location Actor Id)
  (return (Math|Boolean|ANDBoolean (not (AI|IsValidAILocation Location)) (not (Utilities|IsValid Actor)) (== Id "none"))))