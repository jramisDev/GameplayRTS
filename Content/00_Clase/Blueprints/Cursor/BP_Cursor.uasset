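; BP_Cursor is a world-space cursor actor that displays player data through a widget and glides toward a destination location.
; On BeginPlay it casts its widget to WBP_CursorWorld, caches it and initializes it with SPlayerData.
; Each Tick, it uses VInterpTo to ease toward DestinationCursorLocation, teleporting without sweep until within a small tolerance.
; Nothing in this Blueprint sets the destination.
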(event EventBeginPlay
  (bind _aswbp_cursor_world (Utilities|Casting|CastToWBP_CursorWorld (UserInterface|GetWidget (Variables|Default|GetWidget))))
  (bind _output_get (Variables|Default|SetAs%20WBP%20Cursor%20World _aswbp_cursor_world))
  (Default|Init _output_get (Variables|Default|GetS%20Player%20Data)))

(event EventTick
  (params (DeltaSeconds :type Float%20%28single-precision%29))
  (bind _returnvalue (Transformation|GetActorLocation))
  (if (not (Utilities|Operators|EqualEqual _returnvalue (Variables|Default|GetDestination%20Cursor%20Location) 0.2))
    (Transformation|SetActorLocation (Math|Interpolation|VInterpTo _returnvalue (Variables|Default|GetDestination%20Cursor%20Location) DeltaSeconds 1.0) false true)))

(fn ConstructionScript)