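; Construction-site actor for an RTS that stands in for a building until its build time completes, then has GS_RTS spawn the real one and destroys itself.
; On the server, BeginPlay reads grid size and build time from data tables by building ID and scales the grid preview collision to the footprint.
; Each IncreaseWorkingProgress call advances construction; the self-timer, grid snapping and pivot correction are disconnected.
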(event Custom|IncreaseWorkingProgress
  (bind _output_get (Variables|Default|SetCurrentConstructionTime (+ (Variables|Default|GetCurrentConstructionTime) 0.2)))
  (if (>= _output_get (Variables|Default|GetMaxConstructionTime))
    (bind _aspc_rts (Utilities|Casting|CastToPC_RTS (Components|GetOwner)))
    (CallFunction|FinishConstruction _aspc_rts (Variables|Default|GetIDFinalBuilding))))

(event Custom|FinishConstruction
  (params (PC :type PC%20RTS%20Object%20Reference) (ID%20Building :type Name))
  (bind _asgs_rts (Utilities|Casting|CastToGS_RTS (Game|GetGameState)))
  (Default|SpawnBuildforPlayer _asgs_rts PC ID%20Building (Transformation|GetActorLocation) (.color (Variables|/Game/00_Clase/Blueprints/Commons/PC_RTS.PC_RTS_C|GetPlayer%20Data PC)))
  (Actor|DestroyActor))

(event EventBeginPlay
  (Networking|SwitchHasAuthority
    (:Authority
      (bind _returnvalue (Utilities|GetDataTableRow "/Game/00_Clase/Blueprints/Structs/DT_Building.DT_Building" (Variables|Default|GetIDFinalBuilding))
        (:then
          (Variables|Default|SetBuilding%20Size (.gridsize _returnvalue))
          (bind _returnvalue_2 (Utilities|GetDataTableRow "/Game/00_Clase/Blueprints/Structs/DT_Crafteable.DT_Crafteable" (Variables|Default|GetIDFinalBuilding))
            (:then
              (Variables|Default|SetMaxConstructionTime (.time _returnvalue_2))
              (CallFunction|ConstructionScriptThings))))))))

(fn ConstructionScript
  (CallFunction|ConstructionScriptThings))

(fn ClamptoGrid
  (params (InVec :type Vector))
  (bind (_x _y _z) (Math|Vector|BreakVector InVec))
  (Transformation|SetActorLocation (Math|Vector|MakeVector (Math|Conversions|ToFloat(Integer) (* (Math|Float|Round (/ _x 1e+02)) 100)) (Math|Conversions|ToFloat(Integer) (* (Math|Float|Round (/ _y 1e+02)) 100)) _z) false true))

(fn ScaleGridCollision
  (bind _buildinggridpreview (Variables|Default|GetBuildingGridPreview))
  (bind _building_size (Variables|Default|GetBuilding%20Size))
  (bind (_x _y) (Math|Vector2D|BreakVector2D _building_size))
  (Transformation|SetWorldScale3D _buildinggridpreview (Math|Vector|MakeVector _x _y (.z (Transformation|GetWorldScale _buildinggridpreview)))))

(fn CorrectPivotLocation)

(fn ConstructionScriptThings
  (CallFunction|ScaleGridCollision)
  (CallFunction|CorrectPivotLocation))

(fn GetCollisionComponent
  (return (Variables|Default|GetBuildingGridPreview)))

(fn Selected
  (return "" "NewEnumerator10" 0 0))