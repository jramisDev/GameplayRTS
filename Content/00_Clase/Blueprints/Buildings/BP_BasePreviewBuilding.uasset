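; Base building placement preview for an RTS that follows the player's cursor on a grid and shows whether the spot is free.
; Each tick it gets the cursor position from the cached PC_RTS controller and passes it to ClampToGrid.
; A spot counts as buildable when BuildingGridPreview overlaps no actors.
; That result drives the OnOff scalar on a dynamic M_BuildingPreview material created at BeginPlay.
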(event EventBeginPlay
  (|CallParentFunction)
  (bind _returnvalue (Rendering|Material|CreateDynamicMaterialInstance "/Game/00_Clase/Materials/M_BuildingPreview.M_BuildingPreview" "None" "None" :!class /Script/Engine.KismetMaterialLibrary))
  (bind _output_get (Variables|Default|SetMI%20Preview _returnvalue))
  (Rendering|Material|SetMaterial (Variables|Default|GetBuildingGridPreview) 0 _output_get))

(event EventTick
  (params (DeltaSeconds :type Float%20%28single-precision%29))
  (bind _location (Default|GetCursorPosition (CallFunction|GetPCRef) "TraceTypeQuery4"))
  (CallFunction|ClamptoGrid _location)
  (CallFunction|ChangeMaterialColorPreview))

(fn ConstructionScript
  (|CallParentFunction))

(fn GetPCRef
  (Variables|Default|GetAs%20PC%20RTS
    (:then
      _)
    (:else
      (bind _aspc_rts (Utilities|Casting|CastToPC_RTS (Game|GetPlayerController 0)))
      (Variables|Default|SetAs%20PC%20RTS _aspc_rts)))
  (return (Variables|Default|GetAs%20PC%20RTS)))

(fn CanIBuildHere
  (return (Utilities|Array|IsEmpty (Collision|GetOverlappingActors (Variables|Default|GetBuildingGridPreview) 0 :!class /Script/Engine.PrimitiveComponent))))

(fn ChangeMaterialColorPreview
  (Rendering|Material|SetScalarParameterValue (Variables|Default|GetMI%20Preview) "OnOff" (select (CallFunction|CanIBuildHere) 1.0 0.0) :!class /Script/Engine.MaterialInstanceDynamic))