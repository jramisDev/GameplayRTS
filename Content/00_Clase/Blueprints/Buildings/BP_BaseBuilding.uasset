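; Base building actor for an RTS, configured by an element ID that looks up rows in the building, craftable and selection UI DataTables.
; Construction applies the mesh and transform, sizes the grid preview and snaps the actor to a 100-unit grid.
; BeginPlay reloads the data and tints the "PlayerColor" material slot through a dynamic instance.
; It also supplies selection UI data, removes decals on deselect and checks affordability through the local PlayerState.
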(event EventBeginPlay
  (CallFunction|BuildfromDataTable)
  (CallFunction|ChangeColorPlayerMesh))

(event EventDeselect
  (bind _returnvalue (Actor|GetComponentbyClass "/Script/Engine.DecalComponent"))
  (Utilities|IsValid _returnvalue
    (:Is%20Valid
      (Components|DestroyComponent _returnvalue))))

(fn ConstructionScript
  (CallFunction|BuildfromDataTable)
  (CallFunction|SacaleGridCollision)
  (CallFunction|CorrectPivotLocation)
  (CallFunction|ClamptoGrid (Transformation|GetActorLocation)))

(fn ClamptoGrid
  (params (InVec :type Vector))
  (bind (_x _y _z) (Math|Vector|BreakVector InVec))
  (Transformation|SetActorLocation (Math|Vector|MakeVector (Math|Conversions|ToFloat(Integer) (* (Math|Float|Round (/ _x 1e+02)) 100)) (Math|Conversions|ToFloat(Integer) (* (Math|Float|Round (/ _y 1e+02)) 100)) _z) false true))

(fn SacaleGridCollision
  (bind _buildinggridpreview (Variables|Default|GetBuildingGridPreview))
  (bind _building_data (Variables|Default|GetBuilding%20Data))
  (bind (_x _y) (Math|Vector2D|BreakVector2D (.gridsize _building_data)))
  (Transformation|SetWorldScale3D _buildinggridpreview (Math|Vector|MakeVector _x _y (.z (Transformation|GetWorldScale _buildinggridpreview)))))

(fn CorrectPivotLocation
  (bind (_x _y) (Math|Vector2D|BreakVector2D))
  (Transformation|SetRelativeLocation (Variables|Default|GetPositionFixed) (Math|Vector|MakeVector (* _x 5e+01) (* _y 5e+01) 0.0) false false))

(fn BuildfromDataTable
  (bind _meshbuilding (Variables|Default|GetMeshBuilding))
  (Utilities|FlowControl|Sequence
    (:then_0
      (bind _returnvalue (Utilities|GetDataTableRow "/Game/00_Clase/Blueprints/Structs/DT_Building.DT_Building" (Variables|Default|GetID%20Selected%20Element))
        (:then
          (Variables|Default|SetBuilding%20Data _returnvalue)
          (Utilities|FlowControl|Sequence
            (:then_0
              (CallFunction|SacaleGridCollision)
              (CallFunction|CorrectPivotLocation))
            (:then_1
              (Transformation|SetRelativeTransform _meshbuilding (.Transform (Utilities|Struct|BreakS_Building _returnvalue)) false false)
              (Components|StaticMesh|SetStaticMesh _meshbuilding (.Mesh (Utilities|Struct|BreakS_Building _returnvalue))))))))
    (:then_1
      (bind _returnvalue_2 (Utilities|GetDataTableRow "/Game/00_Clase/Blueprints/Structs/DT_Crafteable.DT_Crafteable" (Variables|Default|GetID%20Selected%20Element))
        (:then
          (Variables|Default|SetCrafteableData _returnvalue_2))))
    (:then_2
      (bind _returnvalue_3 (Utilities|GetDataTableRow "/Game/00_Clase/Blueprints/Structs/DT_SelectedElementUI.DT_SelectedElementUI" (Variables|Default|GetID%20Selected%20Element))
        (:then
          (Variables|Default|SetSelected%20UI%20Data _returnvalue_3))))))

(fn ChangeColorPlayerMesh
  (bind _meshbuilding (Variables|Default|GetMeshBuilding))
  (bind _returnvalue (Class|PrimitiveComponent|GetMaterialbyName _meshbuilding "PlayerColor"))
  (Utilities|IsValid _returnvalue
    (:Is%20Valid
      (bind _returnvalue_2 (Rendering|Material|CreateDynamicMaterialInstance _returnvalue "None" "None" :!class /Script/Engine.KismetMaterialLibrary))
      (bind _output_get (Variables|Default|SetMI_ColorBuild _returnvalue_2))
      (Rendering|Material|SetVectorParameterValue _output_get "Color" (Variables|Default|GetColorPlayer) :!class /Script/Engine.MaterialInstanceDynamic)
      (Rendering|Material|SetMaterialbyName (Variables|Default|GetMeshBuilding) "PlayerColor" (Variables|Default|GetMI_ColorBuild)))))

(fn CanIPayIt
  (return (Default|CanIPayIt (CallFunction|GetLocalPSRef) (Utilities|Struct|BreakS_Crafteable (Variables|Default|GetCrafteableData)))))

(fn GetLocalPSRef
  (Variables|Default|GetAs%20PS%20RTS
    (:then
      _)
    (:else
      (bind _asps_rts (Utilities|Casting|CastToPS_RTS (Game|GetPlayerState 0)))
      (Variables|Default|SetAs%20PS%20RTS _asps_rts)))
  (return (Variables|Default|GetAs%20PS%20RTS)))

(fn Selected
  (bind _building_data (Variables|Default|GetBuilding%20Data))
  (bind _selected_ui_data (Variables|Default|GetSelected%20UI%20Data))
  (bind (_transform _mesh _gridsize _attributelist _actionsbuilding _id_crafteable) (Utilities|Struct|BreakS_Building _building_data))
  (bind (_name _description _image _typeselected) (Utilities|Struct|BreakS_SelectedElementsUI _selected_ui_data))
  (return (Utilities|Struct|MakeS_SelectedUIData (Variables|Default|GetID%20Selected%20Element) "NewEnumerator6" _typeselected _image _attributelist) _actionsbuilding _id_crafteable))