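; Rally point actor, stored with the game's buildings, that tints its mesh with the owning player's color.
; On BeginPlay it creates a dynamic material instance from the Cube's first material, if valid, and sets its Color parameter from ColorPlayer.
; The instance is then assigned to the PlayerColor material slot by name, and the construction script only calls the parent's.
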(event EventBeginPlay
  (CallFunction|ChangeColorPlayerMesh))

(fn ConstructionScript
  (|CallParentFunction))

(fn ChangeColorPlayerMesh
  (bind _cube (Variables|Default|GetCube))
  (bind _returnvalue (Rendering|Material|GetMaterial _cube 0))
  (Utilities|IsValid _returnvalue
    (:Is%20Valid
      (bind _returnvalue_2 (Rendering|Material|CreateDynamicMaterialInstance _returnvalue "None" "None" :!class /Script/Engine.KismetMaterialLibrary))
      (bind _output_get (Variables|Default|SetMI_Color _returnvalue_2))
      (Rendering|Material|SetVectorParameterValue _output_get "Color" (Variables|Default|GetColorPlayer) :!class /Script/Engine.MaterialInstanceDynamic)
      (Rendering|Material|SetMaterialbyName (Variables|Default|GetCube) "PlayerColor" (Variables|Default|GetMI_Color)))))