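; Base RTS unit that takes generic orders, moves to its rally point on spawn and supplies UI data, actions and craftables when selected.
; IDUnit looks up its stats, skeletal mesh and selection info in data tables, in both the construction script and BeginPlay.
; The authority spawns and possesses it with an AIC_UnitBase, which receives forwarded orders.
; Attribute changes from the instigating player controller are added to the unit's attributes through ModifyAttributesOnServer.
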(event Custom|ModifyAttributesOnServer
  (params (AttributesArray :type Array%20of%20E_Attribute%20Enums :default "NewEnumerator3") (ValueAttributesArray :type Array%20of%20Floats%20%28double-precision%29))
  (bind _unitdata (Variables|Default|GetUnitData))
  (for (_array_element _array_index) AttributesArray
    (if (.ReturnValue (Utilities|Map|Find (.attributelist _unitdata) _array_element))
      (Utilities|Map|Add (.attributelist _unitdata) _array_element (+ (.Value (Utilities|Map|Find (.attributelist _unitdata) _array_element)) (Utilities|Array|Get(acopy) ValueAttributesArray _array_index))))))

(event EventDeselect
  (bind _returnvalue (Actor|GetComponentbyClass "/Script/Engine.DecalComponent"))
  (Utilities|IsValid _returnvalue
    (:Is%20Valid
      (Components|DestroyComponent _returnvalue))))

(event EventBeginPlay
  (bind _rallypoint (Variables|Default|GetRallyPoint))
  (CallFunction|SpawnAIController)
  (CallFunction|UnitDatafromDataTable)
  (if (Class|KismetMathLibrary|NotEqualExactlyVectorVector _rallypoint "0, 0, 0")
    (AI|AIMoveTo self _rallypoint 0 2e+01 false)))

(event EventModifyAttributes
  (params (PC%20RTS :type PC%20RTS%20Object%20Reference) (AttributeArray :type Array%20of%20E_Attribute%20Enums :default "NewEnumerator3") (ValueAttributeArray :type Array%20of%20Floats%20%28double-precision%29))
  (if (== PC%20RTS (Pawn|GetController (Game|GetInstigator)))
    (CallFunction|ModifyAttributesonServer AttributeArray ValueAttributeArray)))

(event EventGiveGenericOrder
  (params (Order :type E_Actions%20Enum :default "NewEnumerator10") (TargetLocation :type Vector :default "0, 0, 0") (TargetActor :type Actor%20Object%20Reference) (ID :type Name :default "None"))
  (Default|GiveGenericOrder (Variables|Default|GetAI%20Controller) Order TargetLocation TargetActor ID))

(event Custom|SendAnimationStatus
  (params (Animation%20Status :type E_AnimationState%20Enum :default "NewEnumerator0")))

(fn ConstructionScript
  (CallFunction|UnitDatafromDataTable))

(fn UnitDatafromDataTable
  (Utilities|FlowControl|Sequence
    (:then_0
      (bind _returnvalue (Utilities|GetDataTableRow "/Game/00_Clase/Blueprints/Structs/DT_Unit.DT_Unit" (Variables|Default|GetID%20Unit))
        (:then
          (bind _output_get (Variables|Default|SetUnitData _returnvalue))
          (Components|SkeletalMesh|SetSkeletalMeshAsset (Variables|Character|GetMesh) (.Mesh (Utilities|Struct|BreakS_Unit _output_get))))))
    (:then_1
      (bind _returnvalue_2 (Utilities|GetDataTableRow "/Game/00_Clase/Blueprints/Structs/DT_SelectedElementUI.DT_SelectedElementUI" (Variables|Default|GetID%20Unit))
        (:then
          (Variables|Default|SetSelected%20UI%20Data _returnvalue_2))))))

(fn GetAICRef
  (Variables|Default|GetAs%20AI%20Unit%20Base
    (:then
      _)
    (:else
      (bind _asaic_unit_base (Utilities|Casting|CastToAIC_UnitBase (AI|GetAIController self)))
      (Variables|Default|SetAs%20AI%20Unit%20Base _asaic_unit_base)))
  (return (Variables|Default|GetAs%20AI%20Unit%20Base)))

(fn SpawnAIController
  (Networking|SwitchHasAuthority
    (:Authority
      (bind _returnvalue (Game|SpawnActorfromClass "/Game/00_Clase/Blueprints/Units/AIC_UnitBase.AIC_UnitBase_C" (Math|Transform|MakeTransform "0, 0, 0" "0, 0, 0" "1.000000,1.000000,1.000000") "Undefined" "MultiplyWithRoot" (Components|GetOwner) 0))
      (bind _output_get (Variables|Default|SetAI%20Controller _returnvalue))
      (Pawn|Possess _output_get self))))

(fn GetOwnerPC
  (Variables|Default|GetAs%20PC%20RTS
    (:then
      _)
    (:else
      (bind _aspc_rts (Utilities|Casting|CastToPC_RTS (Game|GetInstigatorController)))
      (Variables|Default|SetAs%20PC%20RTS _aspc_rts)))
  (return (Variables|Default|GetAs%20PC%20RTS)))

(fn GetBPARef
  (Variables|Default|GetAs%20ABP%20Villager
    (:then
      _)
    (:else
      (bind _asabp_villager (Utilities|Casting|CastToABP_Villager (Components|SkeletalMesh|GetAnimInstance (Variables|Character|GetMesh))))
      (Variables|Default|SetAs%20ABP%20Villager _asabp_villager)))
  (return (Variables|Default|GetAs%20ABP%20Villager)))

(fn GetCollisionComponent
  (return (Variables|Collision|GetCapsuleComponent)))

(fn Selected
  (bind _unitdata (Variables|Default|GetUnitData))
  (bind _selected_ui_data (Variables|Default|GetSelected%20UI%20Data))
  (bind (_mesh _attributelist _actionsunits _id_crafteable) (Utilities|Struct|BreakS_Unit _unitdata))
  (bind (_name _description _image _typeselected) (Utilities|Struct|BreakS_SelectedElementsUI _selected_ui_data))
  (for _array_element _id_crafteable
    (Utilities|Map|Add (LocalVariables|GetNewLocalVar) _array_element true))
  (return (Utilities|Struct|MakeS_SelectedUIData (Variables|Default|GetID%20Unit) "NewEnumerator6" _typeselected _image _attributelist) _actionsunits (LocalVariables|GetNewLocalVar) 0))