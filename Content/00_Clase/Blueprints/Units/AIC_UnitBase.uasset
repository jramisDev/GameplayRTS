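; Base AI controller for units that receives player orders and runs them through a queue.
; Each action maps to an AI_Module_AC component on the controller, which validates the order, executes it and signals completion to start the next.
; Location-based generic orders replace the queue, while actor orders append to it.
; One special order type picks the first valid action from the Priorities list, despite the "TryRandomOrder" name.
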(event EventGiveOrdertoActor
  (params (Order :type E_Actions%20Enum :default "NewEnumerator10") (Actor :type Actor%20Object%20Reference))
  (bind _modulesavailables (IAConfig|GetAllModules))
  (bind (_value _returnvalue) (Utilities|Map|Find _modulesavailables Order))
  (if _returnvalue
    (bind _yes (Default|IsValidforOrder _value "0.000000,0.000000,-999.000000" Actor "None"))
    (if _yes
      (Orders|AddOrdertoQueue (Utilities|Struct|MakeS_Orders Order "0.000000,0.000000,-999.000000" Actor "None") false))))

(event EventGiveGenericOrder
  (params (Order :type E_Actions%20Enum :default "NewEnumerator10") (TargetLocation :type Vector :default "0, 0, 0") (TargetActor :type Actor%20Object%20Reference) (ID :type Name :default "None"))
  (bind _modulesavailables (IAConfig|GetAllModules))
  (bind (_value _returnvalue) (Utilities|Map|Find _modulesavailables Order))
  (if (Utilities|Enum|Equal(Enum) Order "NewEnumerator10")
    (Orders|TryRandomOrder TargetLocation TargetActor ID)
    (elif _returnvalue
      (bind _yes (Default|IsValidforOrder _value TargetLocation TargetActor ID))
      (if _yes
        (Orders|AddOrdertoQueue (Utilities|Struct|MakeS_Orders (Variables|/Game/00_Clase/Blueprints/Components/AI_Module_AC.AI_Module_AC_C|GetAction _value) TargetLocation TargetActor ID) true)
        (else
          (Development|PrintString "ORDER NOT VALID FOR MODULE" true true "(R=1.000000,G=0.000000,B=0.000000,A=1.000000)")))
      (else
        (Development|PrintString "NOT MODULE AVAILABLE" true true "(R=1.000000,G=0.000000,B=0.000000,A=1.000000)")))))

(event Custom|ResolveNextOrder
  (bind _modulesavailables (Variables|IAConfig|GetModulesAvailables))
  (bind _orders (Variables|Orders|GetOrders))
  (bind _output (Utilities|Array|Get(acopy) _orders))
  (bind (_action _location _actor _id) (Utilities|Struct|BreakS_Orders _output))
  (bind (_value _returnvalue) (Utilities|Map|Find _modulesavailables _action))
  (if (Utilities|Array|IsNotEmpty (Variables|Orders|GetOrders))
    (if _returnvalue
      (bind _yes (Default|IsValidforOrder _value _location _actor _id))
      (if _yes
        (Default|DoYourAction _value _location _actor _id)
        (EventDispatchers|BindEventtoDoneOrder _value (EventDispatchers|CreateEvent :!event Custom|OrderEnded))))))

(event Custom|OrderEnded
  (Utilities|Array|RemoveIndex (Variables|Orders|GetOrders))
  (CallFunction|ResolveNextOrder))

(fn ConstructionScript)

(fn GetUnitRef
  (Variables|Getters|GetAs%20BP%20Base%20Unit
    (:then
      _)
    (:else
      (bind _asbp_base_unit (Utilities|Casting|CastToBP_BaseUnit (Pawn|GetControlledPawn)))
      (Variables|Getters|SetAs%20BP%20Base%20Unit _asbp_base_unit)))
  (return (Variables|Getters|GetAs%20BP%20Base%20Unit)))

(fn GetAllModules
  (if (Utilities|Map|IsEmpty (Variables|IAConfig|GetModulesAvailables))
    (bind _output_get (LocalVariables|SetComponents (Actor|GetComponentsByClass "/Game/00_Clase/Blueprints/Components/AI_Module_AC.AI_Module_AC_C")))
    (for _array_element _output_get
      (Utilities|Map|Add (Variables|IAConfig|GetModulesAvailables) (Variables|/Game/00_Clase/Blueprints/Components/AI_Module_AC.AI_Module_AC_C|GetAction _array_element) _array_element)))
  (return (Variables|IAConfig|GetModulesAvailables)))

(fn TryRandomOrder
  (params (Location :type Vector) (ActorTarget :type Actor%20Object%20Reference) (Id :type Name))
  (bind _array_element (Utilities|Array|ForEachLoopwithBreak (LocalVariables|GetPriorities) :!label _label)
    (:LoopBody
      (if (.ReturnValue (Utilities|Map|Find (IAConfig|GetAllModules) _array_element))
        (bind _yes (Default|IsValidforOrder (.Value (Utilities|Map|Find (IAConfig|GetAllModules) _array_element)) Location ActorTarget Id))
        (if _yes
          (Orders|AddOrdertoQueue (Utilities|Struct|MakeS_Orders _array_element Location ActorTarget Id) true)
          (goto _label Break))))))

(fn AddOrdertoQueue
  (params (NewItem :type S%20Orders%20Structure%20%28by%20ref%29) (RemoveOthers :type Boolean))
  (bind _orders (Variables|Orders|GetOrders))
  (if RemoveOthers
    (CallFunction|OrderEnded)
    (Utilities|Array|Clear (Variables|Orders|GetOrders)))
  (Utilities|Array|Add _orders NewItem)
  (if (== (Utilities|Array|Length _orders) 1)
    (CallFunction|ResolveNextOrder)))