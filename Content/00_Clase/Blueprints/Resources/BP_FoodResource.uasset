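; BP_FoodResource is a selectable food resource actor, one of the game's resource types.
; Its construction script runs the parent's script, then gives the Food mesh a random static mesh picked from the FoodResources array for visual variety.
; Selected returns UI data for the selection panel, using the resource type as ID along with the food texture and attribute list.
; The event graph holds no logic.
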(event EventBeginPlay)

(event Collision|EventActorBeginOverlap
  (params (OtherActor :type Actor%20Object%20Reference)))

(event EventTick
  (params (DeltaSeconds :type Float%20%28single-precision%29)))

(fn ConstructionScript
  (|CallParentFunction)
  (Components|StaticMesh|SetStaticMesh (Variables|Default|GetFood) (.OutItem (Utilities|Array|Random (Variables|Default|GetFoodResources)))))

(fn Selected
  (return (Utilities|Struct|MakeS_SelectedUIData (Utilities|String|StringToName (Utilities|String|EnumtoString (Variables|Default|GetResource%20Type))) "NewEnumerator5" "NewEnumerator3" "/Game/00_Clase/Textures/food.food" (Variables|Default|GetATTRIBUTE%20LIST)) "NewEnumerator0" 0 0))