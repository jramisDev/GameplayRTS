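; BP_TreeResource is a tree resource actor that can describe itself to a selection UI.
; Its construction script runs the parent's, then assigns the Tree component a random mesh from TreeArray for visual variety.
; GetID returns selected-UI data with an ID derived from the resource type enum, fixed resource and selectable types, a wood texture and an attribute list.
; The event graph holds no logic.
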(event EventBeginPlay)

(event Collision|EventActorBeginOverlap
  (params (OtherActor :type Actor%20Object%20Reference)))

(event EventTick
  (params (DeltaSeconds :type Float%20%28single-precision%29)))

(fn ConstructionScript
  (|CallParentFunction)
  (Components|StaticMesh|SetStaticMesh (Variables|Default|GetTree) (.OutItem (Utilities|Array|Random (Variables|Default|GetTreeArray)))))

(fn GetID
  (return (Utilities|Struct|MakeS_SelectedUIData (Utilities|String|StringToName (Utilities|String|EnumtoString (Variables|Default|GetResource%20Type))) "NewEnumerator0" "NewEnumerator3" "/Game/00_Clase/Textures/wood.wood" (Variables|Default|GetATTRIBUTE%20LIST))))