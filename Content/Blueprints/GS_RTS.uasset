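; RTS GameState that syncs player cursor positions through the PC_RTS player controllers.
; BeginPlay starts a looping timer, and SyncPlayersCursor calls SyncCursorForPlayer with each controller's CursorPosition.
; Its nested loop acts only on matching indices, so each controller receives only its own position.
; GetPlayerControllers caches controllers cast from PlayerArray, rebuilding the list when the counts differ.
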(event Custom|SyncPlayersCursor
  (bind _as_pc_rts (CallFunction|GetPlayerControllers))
  (for (_array_element _array_index) _as_pc_rts
    (for (_array_element_2 _array_index_2) _as_pc_rts
      (if (== _array_index _array_index_2)
        (Default|SyncCursorforPlayer _array_element_2 (Variables|/Game/00_Clase/Blueprints/PC_RTS.PC_RTS_C|GetCursorPosition _array_element) _array_element)))))

(event EventBeginPlay
  (Utilities|Time|SetTimerbyEvent (EventDispatchers|CreateEvent :!event Custom|SyncPlayersCursor) 1.0 true))

(fn ConstructionScript)

(fn GetPlayerControllers
  (if (== (Utilities|Array|Length (Variables|Default|GetPlayerArray)) (Utilities|Array|Length (Variables|Default|GetAs%20PC%20RTS)))
    (return (Variables|Default|GetAs%20PC%20RTS))
    (else
      (Utilities|Array|Clear (Variables|Default|GetAs%20PC%20RTS))
      (for _array_element (Variables|Default|GetPlayerArray)
        (bind _aspc_rts (Utilities|Casting|CastToPC_RTS (Game|GetPlayerController _array_element)))
        (Utilities|Array|Add (Variables|Default|GetAs%20PC%20RTS) _aspc_rts))
      (return (Variables|Default|GetAs%20PC%20RTS)))))